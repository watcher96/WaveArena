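; Player character that moves and jumps through Enhanced Input, aims with the mouse and fires rockets.
; Each tick, a visibility trace from the camera along the deprojected cursor direction yaws only the mesh toward the hit point.
; Both fire inputs require grounded movement and spend CPlayerStats energy to spawn the same BP_Rocket, with Fire2 costing twice as much.
; Point damage feeds into CPlayerStats health.
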(event Input|EnhancedActionEvents|EnhancedInputActionIA_Move
  (params (ActionValue :type Vector%202D%20Structure) (ElapsedSeconds :type Float%20%28double-precision%29) (TriggeredSeconds :type Float%20%28double-precision%29) (InputAction :type Input%20Action%20Object%20Reference :default "/Game/Input/IA_Move.IA_Move"))
  (bind (_x _y) (Math|Vector2D|BreakVector2D ActionValue))
  (:Triggered
    (Pawn|Input|AddMovementInput (Math|Vector|MakeVector _x _y 0.0) 1.0 false)))

(event Input|EnhancedActionEvents|EnhancedInputActionIA_Fire2
  (params (ActionValue :type Boolean) (ElapsedSeconds :type Float%20%28double-precision%29) (TriggeredSeconds :type Float%20%28double-precision%29) (InputAction :type Input%20Action%20Object%20Reference :default "/Game/Input/IA_Fire2.IA_Fire2"))
  (:Started
    (if (not (AI|Components|NavMovement|IsFalling (Variables|Character|GetCharacterMovement)))
      (if (> (Variables|/Game/Blueprints/Components/C_PlayerStats.C_PlayerStats_C|GetEnergy (Variables|Default|GetC_PlayerStats)) 8e+01)
        (Default|ModifyEnergy (Variables|Default|GetC_PlayerStats) -8e+01)
        (Game|SpawnActorfromClass "/Game/Blueprints/BP_Rocket.BP_Rocket_C" (Math|Transform|MakeTransform (Transformation|GetWorldLocation (Variables|Default|GetRocketSpawnLocation)) (Transformation|GetWorldRotation (Variables|Character|GetMesh)) "1.000000,1.000000,1.000000") "Undefined" "MultiplyWithRoot" 0 0)))))

(event Input|EnhancedActionEvents|EnhancedInputActionIA_Jump
  (params (ActionValue :type Boolean) (ElapsedSeconds :type Float%20%28double-precision%29) (TriggeredSeconds :type Float%20%28double-precision%29) (InputAction :type Input%20Action%20Object%20Reference :default "/Game/Input/IA_Jump.IA_Jump"))
  (:Started
    (Character|Jump)))

(event Input|EnhancedActionEvents|EnhancedInputActionIA_Fire1
  (params (ActionValue :type Boolean) (ElapsedSeconds :type Float%20%28double-precision%29) (TriggeredSeconds :type Float%20%28double-precision%29) (InputAction :type Input%20Action%20Object%20Reference :default "/Game/Input/IA_Fire1.IA_Fire1"))
  (:Started
    (if (not (AI|Components|NavMovement|IsFalling (Variables|Character|GetCharacterMovement)))
      (if (> (Variables|/Game/Blueprints/Components/C_PlayerStats.C_PlayerStats_C|GetEnergy (Variables|Default|GetC_PlayerStats)) 4e+01)
        (Default|ModifyEnergy (Variables|Default|GetC_PlayerStats) -4e+01)
        (Game|SpawnActorfromClass "/Game/Blueprints/BP_Rocket.BP_Rocket_C" (Math|Transform|MakeTransform (Transformation|GetWorldLocation (Variables|Default|GetRocketSpawnLocation)) (Transformation|GetWorldRotation (Variables|Character|GetMesh)) "1.000000,1.000000,1.000000") "Undefined" "MultiplyWithRoot" 0 0)))))

(event EventBeginPlay
  (Input|AddMappingContext (PlayerController|LocalPlayerSubsystems|GetEnhancedInputLocalPlayerSubsystem (Game|GetPlayerController 0)) "/Game/Input/IMC_Basic.IMC_Basic" 0 "(bIgnoreAllPressedKeysUntilRelease=True,bForceImmediately=False)"))

(event Game|Damage|EventPointDamage
  (params (Damage :type Float%20%28single-precision%29) (DamageType :type Damage%20Type%20Object%20Reference) (HitLocation :type Vector :default "0, 0, 0") (HitNormal :type Vector :default "0, 0, 0") (HitComponent :type Primitive%20Component%20Object%20Reference) (BoneName :type Name :default "None") (ShotFromDirection :type Vector :default "0, 0, 0") (InstigatedBy :type Controller%20Object%20Reference) (DamageCauser :type Actor%20Object%20Reference) (HitInfo :type Hit%20Result%20Structure%20%28by%20ref%29))
  (Default|ModifyHealth (Variables|Default|GetC_PlayerStats) (Math|Float|Truncate Damage)))

(event EventTick
  (params (DeltaSeconds :type Float%20%28single-precision%29))
  (bind _returnvalue (Game|GetPlayerController 0))
  (bind _camera (Variables|Default|GetCamera))
  (bind _mesh (Variables|Character|GetMesh))
  (bind (_locationx _locationy) (Game|Player|GetMousePosition _returnvalue))
  (bind _returnvalue_2 (Transformation|GetWorldLocation _camera))
  (bind _returnvalue_3 (Transformation|GetWorldRotation _mesh))
  (bind (_outhit _returnvalue_4) (Collision|LineTraceByChannel _returnvalue_2 (+ _returnvalue_2 (* (.WorldDirection (Class|GameplayStatics|DeprojectScreentoWorld _returnvalue (Math|Vector2D|MakeVector2D _locationx _locationy))) 100000)) "TraceTypeQuery1" false 0 "None"))
  (if _returnvalue_4
    (Transformation|SetWorldRotation _mesh (Math|Rotator|MakeRotator (.roll _returnvalue_3) (.pitch _returnvalue_3) (.yaw (Math|Rotator|FindLookatRotation (Transformation|GetActorLocation) (.Location (Collision|BreakHitResult _outhit))))) false false)))

(fn ConstructionScript)