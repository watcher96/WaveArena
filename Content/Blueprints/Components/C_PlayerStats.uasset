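; C_PlayerStats is a player stats component that tracks Health and Energy.
; ModifyHealth and ModifyEnergy add a value to their stat without clamping, and ModifyHealth quits the game when Health equals exactly zero.
; Tick regenerates Energy at a fixed rate per second while it is below 100, printing the value each time.
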(event Custom|ModifyHealth
  (params (Value :type Integer))
  (bind _output_get (Variables|Default|SetHealth (+ (Variables|Default|GetHealth) Value)))
  (if (== _output_get 0)
    (Game|QuitGame 0 "Quit" false)))

(event Custom|ModifyEnergy
  (params (Value :type Float%20%28double-precision%29))
  (Variables|Default|SetEnergy (+ (Variables|Default|GetEnergy) Value)))

(event EventTick
  (params (DeltaSeconds :type Float%20%28single-precision%29))
  (if (< (Variables|Default|GetEnergy) 1e+02)
    (bind _output_get (Variables|Default|SetEnergy (+ (* DeltaSeconds 1e+01) (Variables|Default|GetEnergy))))
    (Development|PrintString (Utilities|String|ToString(Float) _output_get))))